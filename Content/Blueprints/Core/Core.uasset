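; Core is an actor with a HealthComponent whose destruction brings up the GameOver widget.
; It caches starting health as the maximum on BeginPlay, then every Tick writes the current health ratio to the Cylinder's "Health" material parameter to drive its color.
; The Destroyed event creates the GameOver widget and adds it to the viewport.
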(event EventBeginPlay
  ;[1 0.4248 0.9481] Begin Play - set max health value
  (Variables|Default|SetMaxHealth (Variables|/Game/Blueprints/HealthComponent.HealthComponent_C|GetHealth (Variables|Default|GetHealthComponent))))

(event EventDestroyed
  ;[0.003806 0 0.2708] Destroy - Game Over binding
  (bind _returnvalue (UserInterface|CreateWidget "/Game/UI/GameOver.GameOver_C"))
  (UserInterface|Viewport|AddtoViewport _returnvalue 0))

(event EventTick
  (params (DeltaSeconds :type Float%20%28single-precision%29))
  ;[0.2917 1 0.6686] Tick - set material parameter, color of cylinder
  (Rendering|Material|SetScalarParameterValueonMaterials (Variables|Default|GetCylinder) "Health" (/ (Variables|/Game/Blueprints/HealthComponent.HealthComponent_C|GetHealth (Variables|Default|GetHealthComponent)) (Variables|Default|GetMaxHealth))))

(fn ConstructionScript)