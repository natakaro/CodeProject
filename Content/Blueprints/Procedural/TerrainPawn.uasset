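; Pawn that lets the player sculpt a MyProceduralTerrain with the mouse, raising it with left click and lowering it with right click.
; Each tick it moves a decal to the cursor's surface hit, aligned to the normal.
; While a button is held, it finds the vertex nearest the decal on the first terrain overlapping its sphere.
; It shifts that vertex's square of neighbors vertically, scaled by delta time, then updates the mesh.
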(event Custom|Build
  ;[1 0.4873 0.4574] Mouse Clicked?
  (if (or (Variables|Default|GetleftMouseButton) (Variables|Default|GetrightMouseButton))
    (Variables|Default|SetnearestVerticeDistance 999999995904.0)
    (Variables|Default|SetnearestVerticeIndex -1)
    (bind _asmy_procedural_terrain (Utilities|Casting|CastToMyProceduralTerrain (Utilities|Array|Get(acopy) (Collision|GetOverlappingActors (Variables|Default|GetSphere) "/Game/Blueprints/Procedural/MyProceduralTerrain.MyProceduralTerrain_C" :!class /Script/Engine.PrimitiveComponent)))) ; Find Procedural Terrain
    ;[1 0.9229 0.2395] Nearest vertice
    (for (_array_element _array_index) (Variables|/Script/ProjectCode.ProceduralTerrain|Getvertices _asmy_procedural_terrain)
      (if (< (Math|Vector|VectorLength (- (Transformation|GetWorldLocation (Variables|Default|GetDecal)) (+ _array_element (Transformation|GetActorLocation _asmy_procedural_terrain)))) (Variables|Default|GetnearestVerticeDistance))
        (Variables|Default|SetnearestVerticeDistance (Math|Vector|VectorLength (- (Transformation|GetWorldLocation (Variables|Default|GetDecal)) (+ _array_element (Transformation|GetActorLocation _asmy_procedural_terrain)))))
        (Variables|Default|SetnearestVerticeIndex _array_index)))
    (if (Utilities|Array|IsValidIndex (Variables|/Script/ProjectCode.ProceduralTerrain|Getvertices _asmy_procedural_terrain) (Variables|Default|GetnearestVerticeIndex))
      ;[0.1963 1 0.362] Neighbors adding height
      (bind _neighbors (Class|ProceduralTerrain|GetNeighbors _asmy_procedural_terrain (Variables|Default|GetnearestVerticeIndex) 3)) ; Get neighbors in square
      (for _array_element_2 _neighbors
        (Utilities|Array|SetArrayElem (Variables|/Script/ProjectCode.ProceduralTerrain|Getvertices _asmy_procedural_terrain) _array_element_2 (+ (Utilities|Array|Get(acopy) (Variables|/Script/ProjectCode.ProceduralTerrain|Getvertices _asmy_procedural_terrain) _array_element_2) (Math|Vector|MakeVector 0.0 0.0 (* (* (Variables|Default|GetdeltaOfLifting) (Utilities|Time|GetWorldDeltaSeconds)) (select (Variables|Default|GetleftMouseButton) 1.0 -1.0))))))
      (Class|ProceduralTerrain|UpdateMesh _asmy_procedural_terrain))))

(event EventBeginPlay
  ;[1 1 1] Beginplay - show cursor
  (Variables|/Script/Engine.PlayerController|SetbShowMouseCursor (Game|GetPlayerController 0) true))

(event EventTick
  (params (DeltaSeconds :type Float%20%28single-precision%29))
  ;[1 1 1] Tick - decal location + build
  (CallFunction|DecalLocationSet)
  (CallFunction|Build))

(event Input|MouseEvents|LeftMouseButton
  (params (Key :type Key%20Structure))
  ;[1 0.2257 0.7713] Input
  (:Pressed
    (Variables|Default|SetleftMouseButton true))
  (:Released
    (Variables|Default|SetleftMouseButton false)))

(event Input|MouseEvents|RightMouseButton
  (params (Key :type Key%20Structure))
  ;[1 0.2257 0.7713] Input
  (:Pressed
    (Variables|Default|SetrightMouseButton true))
  (:Released
    (Variables|Default|SetrightMouseButton false)))

(fn ConstructionScript)

(fn DecalLocationSet
  (bind _returnvalue (Game|GetPlayerController 0))
  (bind _hitresult (Game|Player|GetHitResultUnderCursorbyChannel _returnvalue "TraceTypeQuery1" true))
  (bind (_bblockinghit _binitialoverlap _time _distance _location _impactpoint _normal _impactnormal) (Collision|BreakHitResult _hitresult))
  (Transformation|SetWorldLocationAndRotation (Variables|Default|GetDecal) _location (Math|Rotator|MakeRotationfromAxes _impactnormal "0, 0, 0" "0, 0, 0") false false))