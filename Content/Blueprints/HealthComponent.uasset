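; Actor component that gives its owner health and destroys that owner when health runs out.
; On BeginPlay it binds to the owner's OnTakeAnyDamage event and subtracts incoming damage from Health.
; At zero or below, it clamps Health to zero and calls its Death event, which destroys the owning actor.
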(event Custom|TakeDamage
  (params (DamagedActor :type Actor%20Object%20Reference) (Damage :type Float%20%28single-precision%29) (DamageType :type Damage%20Type%20Object%20Reference) (InstigatedBy :type Controller%20Object%20Reference) (DamageCauser :type Actor%20Object%20Reference))
  ;[1 0.3407 0.3008] Take Damage Binding
  (bind _output_get (Variables|Default|SetHealth (- (Variables|Default|GetHealth) Damage)))
  (if (<= _output_get 0.0)
    (Variables|Default|SetHealth 0.0)
    (CallFunction|Death)))

(event Custom|Death
  ;[0.6332 0.487 1] Death
  (Actor|DestroyActor (Components|GetOwner)))

(event EventBeginPlay
  ;[1 0.3407 0.3008] Take Damage Binding
  (EventDispatchers|BindEventtoOnTakeAnyDamage (Components|GetOwner) (delegate Custom|TakeDamage)))